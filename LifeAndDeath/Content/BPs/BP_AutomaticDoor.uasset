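; Automatic door actor that slides open when the player pawn enters its trigger box and closes when the pawn leaves.
; Overlap events on the Collision box call OpenDoor and CloseDoor, which play and reverse a timeline that lerps the door's relative Z upward, with debug prints.
; The construction script sizes and places the trigger from the TriggerExtents and TriggerLocation variables.
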(event `OpenDoor`
  (bind _door (`self.Door`))
  (bind (_relativelocation_x _relativelocation_y) (`KismetMathLibrary.BreakVector` (`SceneComponent.RelativeLocation` _door)))
  (bind (_direction _alpha) (`Timeline|OpenDoorTimeline` :!label _label)
    (:`Update`
      (`SceneComponent.K2_SetRelativeLocation` _door (`KismetMathLibrary.MakeVector` _relativelocation_x _relativelocation_y (`KismetMathLibrary.Lerp` 0.0 800.0 _alpha)) false false))))

(event `Close Door`
  (goto _label :!via `Reverse`))

(event `self.Collision.OnComponentBeginOverlap`
  (params (OverlappedComponent :type "PrimitiveComponent Object Reference") (OtherActor :type "Actor Object Reference") (OtherComp :type "PrimitiveComponent Object Reference") (OtherBodyIndex :type Integer) (bFromSweep :type Boolean) (SweepResult :type "HitResult Structure (by ref)"))
  (if (== OtherActor (`GameplayStatics.GetPlayerPawn` 0))
    (`self.OpenDoor`)
    (`KismetSystemLibrary.PrintString` "open")))

(event `self.Collision.OnComponentEndOverlap`
  (params (OverlappedComponent :type "PrimitiveComponent Object Reference") (OtherActor :type "Actor Object Reference") (OtherComp :type "PrimitiveComponent Object Reference") (OtherBodyIndex :type Integer))
  (if (== (`GameplayStatics.GetPlayerPawn` 0) OtherActor)
    (`self.Close Door`)
    (`KismetSystemLibrary.PrintString` "close")))

(fn `UserConstructionScript`
  (`BoxComponent.SetBoxExtent` (`self.Collision`) (`self.TriggerExtents`) true)
  (`SceneComponent.K2_SetRelativeLocation` (`self.Collision`) (`self.TriggerLocation`) false false))