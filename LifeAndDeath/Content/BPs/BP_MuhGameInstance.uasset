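; Game instance that carries player progress across levels: last level entered, checkpoint, three powers and level completion.
; Save and load functions copy these values to and from a BP_MuhSaveGame in the fixed slot Save1, while the selected save file is only stored.
; A once-only event loads or creates the save, and deletion rewrites a blank one and reloads.
; Completing a level sets its flag and opens the next, ending at the main menu.
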(event `Update Last Level Entered`
  (params (`Current Level String` :type String))
  ;[1 1 1] Records last level entered
  (set `self.instanceLastLevelEntered` `Current Level String`))

(event `Update Levels Completed`
  (params (`Level Completed String` :type String))
  ;[1 1 1] Update Levels completed bools
  (`KismetSystemLibrary.LogString` `Level Completed String`)
  (switch `string` `Level Completed String`
    (:`The_Shadowyard`
      (set `self.hasCompletedShadowYard` true)
      (`GameplayStatics.OpenLevelBySoftObjectPtr` "/Game/Levels/The_CrystalCity.The_CrystalCity"))
    (:`The_CrystalCity`
      (set `self.hasCompletedCrystalCity` true)
      (`GameplayStatics.OpenLevelBySoftObjectPtr` "/Game/Levels/The_DeathFactory.The_DeathFactory"))
    (:`The_DeathFactory`
      (set `self.hasCompletedDeathFactory` true)
      (`GameplayStatics.OpenLevelBySoftObjectPtr` "/Game/Levels/MainMenu_level.MainMenu_level"))))

(event `Update Instance Checkpoint`
  (params (Location :type "Vector Structure") (LevelName :type String))
  ;[1 1 1] Updates Game instance copy of checkpoint location and the level its associated with
  (set `self.instanceCheckpointLocation` Location)
  (set `self.levelOfCheckpoint` LevelName))

(event `LoadSaveFile`
  ;[1 1 1] Checking if save game exists, then loading or creating save game object
  (`/Engine/EditorBlueprintResources/StandardMacros.DoOnce` false
    (:`Completed`
      (bind _returnvalue (`GameplayStatics.DoesSaveGameExist` (`self.save1`)))
      (if _returnvalue
        (`self.Load My Game`)
        (else
          ;[1 1 1] Create Save File
          (bind _returnvalue_2 (`GameplayStatics.CreateSaveGameObject` "/Game/BPs/BP_MuhSaveGame.BP_MuhSaveGame_C"))
          (`GameplayStatics.SaveGameToSlot` _returnvalue_2 (`self.save1`)))))))

(event `SelectSaveFile`
  (params (saveFileEntered :type String))
  (set `self.chosenSaveFile` saveFileEntered))

(event `DeleteSaveFile`
  ;[1 1 1] Deletes saved file, then has
  (`GameplayStatics.DeleteGameInSlot` (`self.save1`))
  (bind _returnvalue (`GameplayStatics.CreateSaveGameObject` "/Game/BPs/BP_MuhSaveGame.BP_MuhSaveGame_C"))
  (`GameplayStatics.SaveGameToSlot` _returnvalue (`self.save1`))
  (`self.Load My Game`))

(fn `Load My Game`
  (bind _muhsavegameref (`self.MuhSaveGameRef`))
  (bind _muhsavegameref_2 (`self.MuhSaveGameRef`))
  (bind _muhsavegameref_3 (`self.MuhSaveGameRef`))
  ;[1 1 1] Loading game from slot
  (bind _returnvalue (`GameplayStatics.LoadGameFromSlot` (`self.save1`)))
  (bind _asbp_muh_save_game (cast `/Game/BPs/BP_MuhSaveGame` _returnvalue))
  (bind _output_get (set `self.MuhSaveGameRef` _asbp_muh_save_game))
  ;[1 1 1] Setting game instance variables based on save game
  (set `self.instanceLastLevelEntered` (`/Game/BPs/BP_MuhSaveGame.savedLastLevelEntered` _output_get))
  (set `self.instanceCheckpointLocation` (`/Game/BPs/BP_MuhSaveGame.SavedCheckpointLocation` _muhsavegameref))
  (set `self.levelOfCheckpoint` (`/Game/BPs/BP_MuhSaveGame.LevelOfSavedCheckpoint` _muhsavegameref))
  (set `self.hasPower1` (`/Game/BPs/BP_MuhSaveGame.savedHasPower1` _muhsavegameref_2))
  (set `self.hasPower2` (`/Game/BPs/BP_MuhSaveGame.savedHasPower2` _muhsavegameref_2))
  (set `self.hasPower3` (`/Game/BPs/BP_MuhSaveGame.savedHasPower3` _muhsavegameref_2))
  (set `self.hasCompletedShadowYard` (`/Game/BPs/BP_MuhSaveGame.savedCompletedShadowyard` _muhsavegameref_3))
  (set `self.hasCompletedCrystalCity` (`/Game/BPs/BP_MuhSaveGame.savedCompletedCrystalCity` _muhsavegameref_3))
  (set `self.hasCompletedDeathFactory` (`/Game/BPs/BP_MuhSaveGame.savedCompletedDeathFactory` _muhsavegameref_3)))

(fn `Save My Game`
  ;[1 1 1] Loading the existing save file and creating a ref to it
  (bind _returnvalue (`GameplayStatics.LoadGameFromSlot` (`self.save1`)))
  (bind _asbp_muh_save_game (cast `/Game/BPs/BP_MuhSaveGame` _returnvalue))
  (set `self.MuhSaveGameRef` _asbp_muh_save_game)
  ;[1 1 1] Setting save game variables
  (set `/Game/BPs/BP_MuhSaveGame.savedLastLevelEntered` (`self.instanceLastLevelEntered`) _asbp_muh_save_game)
  (set `/Game/BPs/BP_MuhSaveGame.SavedCheckpointLocation` (`self.instanceCheckpointLocation`) (`self.MuhSaveGameRef`))
  (set `/Game/BPs/BP_MuhSaveGame.LevelOfSavedCheckpoint` (`self.levelOfCheckpoint`) (`self.MuhSaveGameRef`))
  (set `/Game/BPs/BP_MuhSaveGame.savedHasPower1` (`self.hasPower1`) (`self.MuhSaveGameRef`))
  (set `/Game/BPs/BP_MuhSaveGame.savedHasPower2` (`self.hasPower2`) (`self.MuhSaveGameRef`))
  (set `/Game/BPs/BP_MuhSaveGame.savedHasPower3` (`self.hasPower3`) (`self.MuhSaveGameRef`))
  (set `/Game/BPs/BP_MuhSaveGame.savedCompletedShadowyard` (`self.hasCompletedShadowYard`) (`self.MuhSaveGameRef`))
  (set `/Game/BPs/BP_MuhSaveGame.savedCompletedCrystalCity` (`self.hasCompletedCrystalCity`) (`self.MuhSaveGameRef`))
  (set `/Game/BPs/BP_MuhSaveGame.savedCompletedDeathFactory` (`self.hasCompletedDeathFactory`) (`self.MuhSaveGameRef`))
  ;[1 1 1] Writing to save file
  (`GameplayStatics.SaveGameToSlot` (`self.MuhSaveGameRef`) (`self.save1`)))