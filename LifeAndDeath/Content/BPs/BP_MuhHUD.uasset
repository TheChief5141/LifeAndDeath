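; BP_MuhHUD is the game's HUD Blueprint, creating the on-screen widgets and handling loading screen fade transitions.
; On BeginPlay it creates and stores the loading screen widget, fades it out, adds the pause button and text display to the viewport, and shows the mouse cursor.
; Two custom events use the stored reference to fade the loading screen in or out.
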(event `HUD transition out Loading Screen`
  ;[1 1 1] Fade out loading Screen
  (`/Game/WBPs/WBP_LoadingScreen.FadeOut Loading Screen` (`self.WBPLoadingScreenRef`)))

(event `HUD transition to Loading Screen`
  ;[1 1 1] Fade in loading Screen
  (`/Game/WBPs/WBP_LoadingScreen.FadeIn Loading Screen` (`self.WBPLoadingScreenRef`)))

(event `self.ReceiveBeginPlay`
  (bind _returnvalue (`GameplayStatics.GetPlayerController` 0))
  ;[1 1 1] Fading into scene from black
  (bind _returnvalue_2 (`|CreateWidget` "/Game/WBPs/WBP_LoadingScreen.WBP_LoadingScreen_C" _returnvalue))
  (bind _output_get (set `self.WBPLoadingScreenRef` _returnvalue_2))
  (`/Game/WBPs/WBP_LoadingScreen.FadeOut Loading Screen` _output_get)
  ;[1 1 1] Adding Pause button to screen
  (bind _returnvalue_3 (`|CreateWidget` "/Game/WBPs/WBP_PauseButton.WBP_PauseButton_C" _returnvalue))
  (`UserWidget.AddToViewport` _returnvalue_3 0)
  (set `PlayerController.bShowMouseCursor` true _returnvalue)
  ;[1 1 1] Adding Text Display Widget (empty by default)
  (bind _returnvalue_4 (`|CreateWidget` "/Game/WBPs/WBP_TextDisplay.WBP_TextDisplay_C" _returnvalue))
  (`UserWidget.AddToViewport` _returnvalue_4 0))

(fn `UserConstructionScript`)