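; BP_MuhPlayerController is the player controller that handles checkpoints, respawning and level progression.
; On BeginPlay it reports the level to the game instance, then moves the pawn to that level's saved checkpoint or clears a stale one.
; Respawning reopens the level, so checkpoints persist through the game instance.
; Reload and next-level events show the HUD loading screen, then open levels chosen by name; DisplayText stores HUD text and speed.
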(event `self.ReceiveBeginPlay`
  (bind _muhgameinstanceref (`self.MuhGameInstanceRef`))
  ;[1 1 1] Saving HUD Ref
  (bind _asbp_muh_hud (cast `/Game/BPs/BP_MuhHUD` (`self.GetHUD`)))
  (set `self.As BP Muh HUD` _asbp_muh_hud)
  ;[1 1 1] Saving game instance ref
  (bind _asbp_muh_game_instance (cast `/Game/BPs/BP_MuhGameInstance` (`GameplayStatics.GetGameInstance`)))
  (set `self.MuhGameInstanceRef` _asbp_muh_game_instance)
  ;[1 1 1] Record name of current level as string and pass this to game instance
  (bind _returnvalue (`GameplayStatics.GetCurrentLevelName` true))
  (bind _output_get (set `self.currentLevelName` _returnvalue))
  (`/Game/BPs/BP_MuhGameInstance.Update Last Level Entered` (`self.MuhGameInstanceRef`) _output_get)
  ;[1 1 1] Depending on if the game instance checkpoint's level matches the current level
  (if (`KismetStringLibrary.EqualEqual_StrStr` (`self.currentLevelName`) (`/Game/BPs/BP_MuhGameInstance.levelOfCheckpoint` (`self.MuhGameInstanceRef`)))
    ;[1 1 1] Set the current checkpoint to the game instance checkpoint
    (set `self.PlayerSpawnLocation` (`/Game/BPs/BP_MuhGameInstance.instanceCheckpointLocation` (`self.MuhGameInstanceRef`)))
    (`self.K2_SetActorLocation` (`GameplayStatics.GetPlayerPawn` 0) (`self.PlayerSpawnLocation`) false false)
    (else
      ;[1 1 1] Sets the level of the game instance checkpoint to empty and its location to 0,0,0
      (set `/Game/BPs/BP_MuhGameInstance.levelOfCheckpoint` "" _muhgameinstanceref)
      (set `/Game/BPs/BP_MuhGameInstance.instanceCheckpointLocation` (0.0 0.0 0.0) _muhgameinstanceref)
      (`KismetSystemLibrary.PrintString` "old checkpoint cleared"))))

(event `Respawn`
  ;[1 1 1] Respawning character at spawn location
  (`self.Reopen Level`))

(event `Reopen Level`
  ;[1 1 1] Reopening current level
  (`/Game/BPs/BP_MuhHUD.HUD transition to Loading Screen` (`self.As BP Muh HUD`))
  (`KismetSystemLibrary.Delay` 1.0)
  (switch `string` (`self.currentLevelName`)
    (:`The_Shadowyard`
      (`GameplayStatics.OpenLevelBySoftObjectPtr` "/Game/Levels/The_Shadowyard.The_Shadowyard"))
    (:`The_CrystalCity`
      (`GameplayStatics.OpenLevelBySoftObjectPtr` "/Game/Levels/The_CrystalCity.The_CrystalCity"))
    (:`The_DeathFactory`
      (`GameplayStatics.OpenLevelBySoftObjectPtr` "/Game/Levels/The_DeathFactory.The_DeathFactory"))))

(event `SetNewSpawnLocation`
  (params (NewSpawnLocation :type "Vector Structure"))
  ;[1 1 1] Updating Spawn Location
  (bind _output_get (set `self.PlayerSpawnLocation` NewSpawnLocation))
  (`/Game/BPs/BP_MuhGameInstance.Update Instance Checkpoint` (`self.MuhGameInstanceRef`) _output_get (`self.currentLevelName`)))

(event `LoadNextLevel`
  ;[1 1 1] Plays Loading Screen anim and opens next level
  (`/Game/BPs/BP_MuhHUD.HUD transition to Loading Screen` (`self.As BP Muh HUD`))
  (`KismetSystemLibrary.Delay` 1.0)
  (switch `string` (`self.currentLevelName`)
    (:`The_Shadowyard`
      (`GameplayStatics.OpenLevelBySoftObjectPtr` "/Game/Levels/The_CrystalCity.The_CrystalCity"))
    (:`The_CrystalCity`
      (`GameplayStatics.OpenLevelBySoftObjectPtr` "/Game/Levels/The_DeathFactory.The_DeathFactory"))
    (:`The_DeathFactory`
      (`GameplayStatics.OpenLevelBySoftObjectPtr` "/Game/Levels/MainMenu_level.MainMenu_level"))))

(event `/Game/BPs/BPIs/BPI_DisplayText.DisplayText`
  (params (TextToDisplay :type String) (PlaybackSpeed :type "Float (double-precision)"))
  ;[1 1 1] Updates text values to display in HUD
  (set `self.HUDText` (`KismetTextLibrary.Conv_StringToText` TextToDisplay))
  (set `self.TextSpeed` PlaybackSpeed))

(fn `UserConstructionScript`)