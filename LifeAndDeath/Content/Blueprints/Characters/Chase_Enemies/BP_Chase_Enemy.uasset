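; Chase enemy that pursues the player on sight and defeats PZD_Player_Ken on contact.
; PawnSensing sets AnimState on any sighting and starts an AI MoveTo toward the player character if the seen pawn's class matches.
; Box overlap disables Ken's movement, swaps all cached Paper2D sprites and flipbooks to Crystal Enemy attack and idle assets respectively, then calls PlayerDefeat after a short delay.
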(event `self.ReceiveBeginPlay`
  (set `self.Still_Array` (`|MakeArray` (`self.PaperSprite3`) (`self.PaperSprite2`) (`self.PaperSprite1`) (`self.PaperSprite`)))
  (set `self.Anim_Array` (`|MakeArray` (`self.PaperFlipbook4`) (`self.PaperFlipbook3`) (`self.PaperFlipbook2`) (`self.PaperFlipbook1`) (`self.PaperFlipbook`))))

(event `self.PawnSensing.OnSeePawn`
  (params (Pawn :type "Pawn Object Reference"))
  (bind _returnvalue (`GameplayStatics.GetPlayerCharacter` 0))
  (set `self.Anim_State` 1)
  (if (`KismetMathLibrary.ClassIsChildOf` (`GameplayStatics.GetObjectClass` Pawn) (`GameplayStatics.GetObjectClass` _returnvalue))
    (`|AIMoveTo` self (0.0 0.0 0.0) _returnvalue
      (:`then`
        (`KismetSystemLibrary.PrintString` "seen")))))

(event `self.Box.OnComponentBeginOverlap`
  (params (OverlappedComponent :type "PrimitiveComponent Object Reference") (OtherActor :type "Actor Object Reference") (OtherComp :type "PrimitiveComponent Object Reference") (OtherBodyIndex :type Integer) (bFromSweep :type Boolean) (SweepResult :type "HitResult Structure (by ref)"))
  (if (`KismetMathLibrary.ClassIsChildOf` (`GameplayStatics.GetObjectClass` OtherActor) "/Game/Blueprints/Characters/PlayerCharacter/PZD_Player_Ken.PZD_Player_Ken_C")
    (bind _aspzd_player_ken (cast `/Game/Blueprints/Characters/PlayerCharacter/PZD_Player_Ken` OtherActor))
    (`CharacterMovementComponent.DisableMovement` (`Character.CharacterMovement` _aspzd_player_ken))
    (for _array_element (`self.Still_Array`)
      (`PaperSpriteComponent.SetSprite` _array_element "/Game/Art/Crystal_Buddy/Attack/Crystal_Enemy_Attack_5_Sprite_0.Crystal_Enemy_Attack_5_Sprite_0"))
    (for _array_element_2 (`self.Anim_Array`)
      (`PaperFlipbookComponent.SetFlipbook` _array_element_2 "/Game/Art/Crystal_Buddy/Idle/Crystal_Enemy_Idle_Anim.Crystal_Enemy_Idle_Anim"))
    (`KismetSystemLibrary.Delay` 0.8)
    (`/Game/Blueprints/Characters/PlayerCharacter/PZD_Player_Ken.PlayerDefeat` _aspzd_player_ken)))

(fn `UserConstructionScript`)