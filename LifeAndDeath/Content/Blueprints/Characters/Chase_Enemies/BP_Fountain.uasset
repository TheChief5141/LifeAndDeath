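; BP_Fountain is a fountain actor whose static mesh is revealed when the Ken player reaches it in the DEATH character state.
; The construction script hides the mesh if the game instance's PlayerCharacterState is DEATH.
; On box overlap by a PZD_Player_Ken or child class, it checks that state again and makes the mesh visible if it is DEATH.
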(event `self.Box.OnComponentBeginOverlap`
  (params (OverlappedComponent :type "PrimitiveComponent Object Reference") (OtherActor :type "Actor Object Reference") (OtherComp :type "PrimitiveComponent Object Reference") (OtherBodyIndex :type Integer) (bFromSweep :type Boolean) (SweepResult :type "HitResult Structure (by ref)"))
  (if (`KismetMathLibrary.ClassIsChildOf` (`GameplayStatics.GetObjectClass` OtherActor) "/Game/Blueprints/Characters/PlayerCharacter/PZD_Player_Ken.PZD_Player_Ken_C")
    (switch `/Game/Blueprints/Characters/BP_Player_Char_Enum` (`/Game/BPs/BP_MuhGameInstance.PlayerCharacterState` (cast `/Game/BPs/BP_MuhGameInstance` (`GameplayStatics.GetGameInstance`) :!pure true))
      (:`NewEnumerator1`
        (`SceneComponent.SetVisibility` (`self.StaticMesh`) true false)))))

(fn `UserConstructionScript`
  (switch `/Game/Blueprints/Characters/BP_Player_Char_Enum` (`/Game/BPs/BP_MuhGameInstance.PlayerCharacterState` (cast `/Game/BPs/BP_MuhGameInstance` (`GameplayStatics.GetGameInstance`) :!pure true))
    (:`NewEnumerator1`
      (`SceneComponent.SetVisibility` (`self.StaticMesh`) false false))))