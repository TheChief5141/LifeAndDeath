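; Crystal enemy character with Paper2D flipbook visuals that chases the player on sight and defeats PZD_Player_Ken on box overlap.
; PawnSensing starts an AIMoveTo toward the player character; a custom roam event moves to random reachable nearby points, retriggering roaming on success.
; It begins in a wait flipbook, and a stop event switches to a sleep flipbook while resetting the walking and animation state.
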(event `self.ReceiveBeginPlay`
  (set `self.Anim_State` 0)
  (set `MovementComponent.Velocity` (2.0 2.0 2.0) (`self.CharacterMovement`))
  (`PaperFlipbookComponent.SetFlipbook` (`self.PaperFlipbook`) "/Game/Art/Crystal_Buddy/Attack/Crystal_Wait.Crystal_Wait"))

(event `self.Box.OnComponentBeginOverlap`
  (params (OverlappedComponent :type "PrimitiveComponent Object Reference") (OtherActor :type "Actor Object Reference") (OtherComp :type "PrimitiveComponent Object Reference") (OtherBodyIndex :type Integer) (bFromSweep :type Boolean) (SweepResult :type "HitResult Structure (by ref)"))
  (if (`KismetMathLibrary.ClassIsChildOf` (`GameplayStatics.GetObjectClass` OtherActor) "/Game/Blueprints/Characters/PlayerCharacter/PZD_Player_Ken.PZD_Player_Ken_C")
    (bind _aspzd_player_ken (cast `/Game/Blueprints/Characters/PlayerCharacter/PZD_Player_Ken` OtherActor))
    (`/Game/Blueprints/Characters/PlayerCharacter/PZD_Player_Ken.PlayerDefeat` _aspzd_player_ken)))

(event `Stop_Moving`
  (set `self.IsWalking` false)
  (set `self.Anim_State` 0)
  (`PaperFlipbookComponent.SetFlipbook` (`self.PaperFlipbook`) "/Game/Art/Crystal_Buddy/Attack/Crystal_Enemy_Sleep_Anim.Crystal_Enemy_Sleep_Anim"))

(event `Random_Roam`
  (set `self.Anim_State` 1)
  (set `self.IsWalking` true)
  (`|AIMoveTo` self (`NavigationSystemV1.K2_GetRandomReachablePointInRadius` (`self.K2_GetActorLocation`) 1500.0 null null) null
    (:`OnSuccess`
      (`self.Random_Roam`))))

(event `self.PawnSensing.OnSeePawn`
  (params (Pawn :type "Pawn Object Reference"))
  (bind _returnvalue (`GameplayStatics.GetPlayerCharacter` 0))
  (set `self.Anim_State` 1)
  (if (`KismetMathLibrary.ClassIsChildOf` (`GameplayStatics.GetObjectClass` Pawn) (`GameplayStatics.GetObjectClass` _returnvalue))
    (`|AIMoveTo` self (0.0 0.0 0.0) _returnvalue)))

(fn `UserConstructionScript`)