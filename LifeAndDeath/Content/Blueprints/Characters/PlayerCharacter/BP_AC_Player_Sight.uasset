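; Player sight component that models eye hydration and blinking and tracks whether the player can see.
; A one-shot BeginPlay timer calls Hydration_Loop, which waits at full hydration or otherwise drains it, blinking at empty.
; Blink shows a WBP_Blink widget holding a reference to the component, and End_Blink refills hydration and re-arms blinking.
; Tick clears CanSee while blinking or in darkness without a flashlight.
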(event `self.ReceiveBeginPlay`
  (`KismetSystemLibrary.K2_SetTimerDelegate` (delegate `Hydration_Loop`) 1.0))

(event `Hydration_Loop`
  ;[1 1 1] Eye Hydration Level Loop
  (if (== (`self.EyeHydrationMax`) (`self.EyeHydration`))
    (`/Engine/EditorBlueprintResources/StandardMacros.DoOnce` false :!label _label
      (:`Completed`
        (`KismetSystemLibrary.Delay` (`self.Hydration_Delay`))))
    (else
      (`|ExecutionSequence`
        (:`then_0`
          (goto _label :!via `Reset`))
        (:`then_1`
          (bind _output_get (set `self.EyeHydration` (- (`self.EyeHydration`) (`self.Hydration_Drain`))))
          (if (<= _output_get 0.0)
            (`self.Blink`)))))))

(event `Blink`
  ;[1 1 1] Blinking
  (`/Engine/EditorBlueprintResources/StandardMacros.DoOnce` false :!label _label_2
    (:`Completed`
      (set `self.Blinking` true)
      (bind _returnvalue (`|CreateWidget` "/Game/WBPs/WBP_Blink.WBP_Blink_C" (`GameplayStatics.GetPlayerController` 0)))
      (set `/Game/WBPs/WBP_Blink.BlinkComponent` self _returnvalue)
      (`UserWidget.AddToViewport` _returnvalue 0))))

(event `End_Blink`
  ;[1 1 1] Blinking
  (set `self.Blinking` false)
  (set `self.EyeHydration` (`self.EyeHydrationMax`))
  (goto _label_2 :!via `Reset`))

(event `self.ReceiveTick`
  (params (DeltaSeconds :type "Float (single-precision)"))
  ;[1 1 1] Set Can See
  (set `self.CanSee` (not (or (and (`self.Dark`) (not (`self.Flashlight`))) (`self.Blinking`)))))