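; AI controller for the Shadow character that scans for the player by spinning its possessed pawn.
; Every Tick, BeginSearch yaws the pawn's root component at a rate scaled by delta time and a yaw multiplier.
; AI Perception updates trigger the attack event when the perceived actor is a PZD_Player_Ken, without checking whether it was sensed or lost.
; The attack is a placeholder that only prints a debug message.
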(event `self.ReceiveBeginPlay`)

(event `self.ReceivePossess`
  (params (PossessedPawn :type "Pawn Object Reference"))
  (set `self.Possessed Pawn` PossessedPawn))

(event `self.ReceiveTick`
  (params (DeltaSeconds :type "Float (single-precision)"))
  (`self.BeginSearch` DeltaSeconds (`self.Possessed Pawn`)))

(event `BeginSearch`
  (params (`Yaw Multiplier` :type "Float (double-precision)") (Rotating_Object :type "Actor Object Reference"))
  (`SceneComponent.K2_AddLocalRotation` (`Actor.RootComponent` Rotating_Object) (`KismetMathLibrary.MakeRotator` 0.0 0.0 (* `Yaw Multiplier` (`self.YawMultipier`))) false false))

(event `Attack_Player`
  (params (Player_Actor :type "Actor Object Reference"))
  (`KismetSystemLibrary.PrintString` "seen"))

(event `self.AIPerception.OnTargetPerceptionUpdated`
  (params (Actor :type "Actor Object Reference") (Stimulus :type "AIStimulus Structure"))
  (bind _output_get (set `self.Perceived_Actor` Actor))
  (if (`KismetMathLibrary.ClassIsChildOf` (`GameplayStatics.GetObjectClass` _output_get) "/Game/Blueprints/Characters/PlayerCharacter/PZD_Player_Ken.PZD_Player_Ken_C")
    (`self.Attack_Player` _output_get)))

(fn `UserConstructionScript`)