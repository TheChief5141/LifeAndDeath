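; Collectible power pickup, configured per instance as Fire, Tree or Life, that unlocks that power for the player.
; On BeginPlay, the power name picks the Paper2D sprite and its tint.
; When the player character PZD_Player_Ken overlaps the box, it sets the matching power flag on the player and records the unlock in BP_MuhGameInstance, then destroys itself.
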(event `self.ReceiveBeginPlay`
  (bind _papersprite (`self.PaperSprite`))
  (bind _papersprite_2 (`self.PaperSprite`))
  ;[1 1 1] Switching sprite and its color depending on Name given per instance
  (switch `string` (`self.Name_Of_Power`)
    (:`Fire`
      (`PaperSpriteComponent.SetSprite` _papersprite_2 "/Game/Images/NPC/Flames_Sprite_0.Flames_Sprite_0")
      (`PaperSpriteComponent.SetSpriteColor` _papersprite (`self.FireColor`)))
    (:`Tree`
      (`PaperSpriteComponent.SetSprite` _papersprite_2 "/Game/Images/NPC/Baby_Birds_for_Park_Sprite_0.Baby_Birds_for_Park_Sprite_0")
      (`PaperSpriteComponent.SetSpriteColor` _papersprite (`self.TreeColor`)))
    (:`Life`
      (`PaperSpriteComponent.SetSprite` _papersprite_2 "/Game/Images/NPC/Circle_Creature_2_Sprite_0.Circle_Creature_2_Sprite_0")
      (`PaperSpriteComponent.SetSpriteColor` _papersprite (`self.LifeColor`)))))

(event `self.Box.OnComponentBeginOverlap`
  (params (OverlappedComponent :type "PrimitiveComponent Object Reference") (OtherActor :type "Actor Object Reference") (OtherComp :type "PrimitiveComponent Object Reference") (OtherBodyIndex :type Integer) (bFromSweep :type Boolean) (SweepResult :type "HitResult Structure (by ref)"))
  (bind _returnvalue (`GameplayStatics.GetGameInstance`))
  (bind _returnvalue_2 (`GameplayStatics.GetPlayerCharacter` 0))
  ;[1 1 1] Checking if colliding object is the player
  (bind _output_get (set `self.Hit_Collectible` OtherActor))
  (if (`KismetMathLibrary.ClassIsChildOf` (`GameplayStatics.GetObjectClass` _output_get) "/Game/Blueprints/Characters/PlayerCharacter/PZD_Player_Ken.PZD_Player_Ken_C")
    ;[1 1 1] Checking the instanced name of this collectable
    (switch `string` (`self.Name_Of_Power`)
      (:`Fire`
        (bind _aspzd_player_ken (cast `/Game/Blueprints/Characters/PlayerCharacter/PZD_Player_Ken` _returnvalue_2))
        (set `/Game/Blueprints/Characters/PlayerCharacter/PZD_Player_Ken.Has_Fire` true _aspzd_player_ken)
        ;[1 1 1] Setting bool in game instance for powers unlocked
        (bind _asbp_muh_game_instance (cast `/Game/BPs/BP_MuhGameInstance` _returnvalue))
        (set `/Game/BPs/BP_MuhGameInstance.hasPower1` true _asbp_muh_game_instance))
      (:`Tree`
        (bind _aspzd_player_ken_2 (cast `/Game/Blueprints/Characters/PlayerCharacter/PZD_Player_Ken` _returnvalue_2))
        (set `/Game/Blueprints/Characters/PlayerCharacter/PZD_Player_Ken.Has_Tree` true _aspzd_player_ken_2)
        (bind _asbp_muh_game_instance_2 (cast `/Game/BPs/BP_MuhGameInstance` _returnvalue))
        (set `/Game/BPs/BP_MuhGameInstance.hasPower2` true _asbp_muh_game_instance_2))
      (:`Life`
        (bind _aspzd_player_ken_3 (cast `/Game/Blueprints/Characters/PlayerCharacter/PZD_Player_Ken` _returnvalue_2))
        (set `/Game/Blueprints/Characters/PlayerCharacter/PZD_Player_Ken.Has_Life` true _aspzd_player_ken_3)
        (bind _asbp_muh_game_instance_3 (cast `/Game/BPs/BP_MuhGameInstance` _returnvalue))
        (set `/Game/BPs/BP_MuhGameInstance.hasPower3` true _asbp_muh_game_instance_3)))
    (`self.K2_DestroyActor`)))

(fn `UserConstructionScript`)