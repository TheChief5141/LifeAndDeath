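; BP_Collectible_Story is a story collectible that registers itself when the player touches it.
; The construction script picks the Paper2D sprite from NameOfCollectible, defaulting to a chef hat; the open and closed locket names map to the opposite-named sprites.
; On box overlap by a PZD_Player_Ken actor, it adds that name to BP_MuhGameInstance's collectible list, without destroying or hiding itself.
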(event `self.ReceiveBeginPlay`)

(event `self.Box.OnComponentBeginOverlap`
  (params (OverlappedComponent :type "PrimitiveComponent Object Reference") (OtherActor :type "Actor Object Reference") (OtherComp :type "PrimitiveComponent Object Reference") (OtherBodyIndex :type Integer) (bFromSweep :type Boolean) (SweepResult :type "HitResult Structure (by ref)"))
  (if (`KismetMathLibrary.ClassIsChildOf` (`GameplayStatics.GetObjectClass` OtherActor) "/Game/Blueprints/Characters/PlayerCharacter/PZD_Player_Ken.PZD_Player_Ken_C")
    (bind _asbp_muh_game_instance (cast `/Game/BPs/BP_MuhGameInstance` (`GameplayStatics.GetGameInstance`)))
    (`/Game/BPs/BP_MuhGameInstance.Add_Collectible_To_List` _asbp_muh_game_instance (`self.NameOfCollectible`))))

(fn `UserConstructionScript`
  (bind _papersprite (`self.PaperSprite`))
  (switch `string` (`self.NameOfCollectible`)
    (:`Default`
      (`PaperSpriteComponent.SetSprite` _papersprite "/Game/Art/Collectible_Art_Assets/Collectible_Hats/ChefHat_Sprite_0.ChefHat_Sprite_0"))
    (:`Heart_Locket_Open`
      (`PaperSpriteComponent.SetSprite` _papersprite (`self.Closed_Locket`)))
    (:`Heart_Locket_Closed`
      (`PaperSpriteComponent.SetSprite` _papersprite (`self.Open_Locket`)))
    (:`Cookie_and_Flower`
      (`PaperSpriteComponent.SetSprite` _papersprite (`self.Cookie_Flower`)))))