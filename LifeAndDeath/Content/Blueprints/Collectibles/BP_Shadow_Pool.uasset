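; Shadow pool collectible actor that builds up a ShadowAmount counter while the AB_Player_Death character overlaps its Plane.
; Overlap begin starts a looping one-second timer that increments the counter and calls an end-timer event once it reaches ten.
; Overlap end re-sets the same timer as non-looping rather than clearing it, allowing one final increment.
; The End_Timer event is empty, so nothing stops the count at the limit.
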(event `self.Plane.OnComponentBeginOverlap`
  (params (OverlappedComponent :type "PrimitiveComponent Object Reference") (OtherActor :type "Actor Object Reference") (OtherComp :type "PrimitiveComponent Object Reference") (OtherBodyIndex :type Integer) (bFromSweep :type Boolean) (SweepResult :type "HitResult Structure (by ref)"))
  (if (`KismetMathLibrary.ClassIsChildOf` (`GameplayStatics.GetObjectClass` OtherActor) "/Game/Blueprints/Characters/Death/AB_Player_Death.AB_Player_Death_C")
    (`KismetSystemLibrary.K2_SetTimerDelegate` (delegate `Start_Shadow_Timer`) 1.0 true)))

(event `Start_Shadow_Timer`
  (bind _result (`/Engine/EditorBlueprintResources/StandardMacros.IncrementInt` (`self.Shadow_Amount`))
    (:`  `
      (if (not (< _result 10))
        (`self.End_Timer`)))))

(event `self.Plane.OnComponentEndOverlap`
  (params (OverlappedComponent :type "PrimitiveComponent Object Reference") (OtherActor :type "Actor Object Reference") (OtherComp :type "PrimitiveComponent Object Reference") (OtherBodyIndex :type Integer))
  (if (`KismetMathLibrary.ClassIsChildOf` (`GameplayStatics.GetObjectClass` OtherActor) "/Game/Blueprints/Characters/Death/AB_Player_Death.AB_Player_Death_C")
    (`KismetSystemLibrary.K2_SetTimerDelegate` (delegate `Start_Shadow_Timer`) 1.0)))

(event `End_Timer`)

(fn `UserConstructionScript`)