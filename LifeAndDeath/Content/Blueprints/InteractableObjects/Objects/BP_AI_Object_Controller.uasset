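; Controller for interactable objects that opens a power selection UI when an object is clicked.
; Its click handler records the touched actor on the player (PZD_Player_Ken) if it implements BI_Interactable.
; If the game instance reports any of three powers, it spawns a BP_PWS_Actor offset from and owned by that object.
; It then shows that actor's widget and focuses game-and-UI input on it.
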(event `OnClicked_Event`
  (params (TouchedActor :type "Actor Object Reference") (ButtonPressed :type "Key Structure" :default "None"))
  (bind _clicked_interactable_object (`self.Clicked_Interactable_Object`))
  ;[1 1 1] On clicked, setting the clicked actor, and getting its transform
  (if (not (== (`self.Power_Widget`) "/Game/Blueprints/Widgets/WB_Power_Select.WB_Power_Select"))
    (set `self.Clicked_Interactable_Object` TouchedActor)
    (bind _output_get (set `self.Out Transform` (`self.GetTransform` _clicked_interactable_object)))
    ;[1 1 1] If it has the interactable interface, cast to player and check if they have *any* power
    (if (`KismetSystemLibrary.DoesImplementInterface` _clicked_interactable_object "/Game/Blueprints/InteractableObjects/Interfaces/BI_Interactable.BI_Interactable_C")
      (bind _asbp_muh_game_instance (cast `/Game/BPs/BP_MuhGameInstance` (`GameplayStatics.GetGameInstance`)))
      (bind _aspzd_player_ken (cast `/Game/Blueprints/Characters/PlayerCharacter/PZD_Player_Ken` (`GameplayStatics.GetPlayerCharacter` 0)))
      (set `/Game/Blueprints/Characters/PlayerCharacter/PZD_Player_Ken.Clicked_Actor` (`self.Clicked_Interactable_Object`) _aspzd_player_ken)
      (if (or (`/Game/BPs/BP_MuhGameInstance.hasPower1` _asbp_muh_game_instance) (`/Game/BPs/BP_MuhGameInstance.hasPower2` _asbp_muh_game_instance) (`/Game/BPs/BP_MuhGameInstance.hasPower3` _asbp_muh_game_instance))
        ;[1 1 1] Spawn interactable PWS UI actor, make it owned by the clicked object, and make it visible
        (bind _returnvalue (`|SpawnActorFromClass` "/Game/Blueprints/InteractableObjects/Objects/BP_PWS_Actor.BP_PWS_Actor_C" (`KismetMathLibrary.MakeTransform` (+ (.location _output_get) (0.0 75.0 0.0)) (.rotation _output_get) (.scale _output_get)) "Undefined" "MultiplyWithRoot" null null))
        (`self.SetOwner` _returnvalue (`self.Clicked_Interactable_Object`))
        (bind _widget (`/Game/Blueprints/InteractableObjects/Objects/BP_PWS_Actor.Widget` _returnvalue))
        (`SceneComponent.SetVisibility` _widget true false)
        (bind _output_get_2 (set `self.Power_Widget` (`WidgetComponent.GetWidget` _widget)))
        (`WidgetBlueprintLibrary.SetInputMode_GameAndUIEx` (`GameplayStatics.GetPlayerController` 0) _output_get_2 "DoNotLock" false)))))

(fn `UserConstructionScript`)