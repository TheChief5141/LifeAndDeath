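; BP_Box is a clickable interactable box with its own controller that can respond to powers.
; Clicks bound on BeginPlay are forwarded to its BP_AI_Object_Controller as left-button clicks.
; Create_Fire spawns BP_Power_Fire at the player character, issues it a move whose goal is itself, then destroys the box.
; RunInteraction only prints the power used, while Add_Tree and Grant_Life are empty stubs.
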(event `self.ReceiveBeginPlay`
  (add `self.OnClicked` (delegate `OnClicked_Event`)))

(event `/Game/Blueprints/InteractableObjects/Interfaces/BI_Interactable.RunInteraction`
  (params (PowerUsed :type Byte))
  (`KismetSystemLibrary.PrintString` (`KismetStringLibrary.Conv_ByteToString` PowerUsed)))

(event `OnClicked_Event` :!signature `self.OnClicked`
  (params (TouchedActor :type "Actor Object Reference") (ButtonPressed :type "Key Structure" :default "None"))
  (bind _asbp_ai_object_controller (cast `/Game/Blueprints/InteractableObjects/Objects/BP_AI_Object_Controller` (`self.GetController`))
    (:`then`
      (`/Game/Blueprints/InteractableObjects/Objects/BP_AI_Object_Controller.OnClicked_Event` _asbp_ai_object_controller self "LeftMouseButton"))
    (:`CastFailed`
      (`KismetSystemLibrary.PrintString` "failed"))))

(event `Create_Fire`
  (params (Clicked_Object :type "Actor Object Reference"))
  (bind _returnvalue (`|SpawnActorFromClass` "/Game/Blueprints/Powers/BP_Power_Fire.BP_Power_Fire_C" (`SceneComponent.K2_GetComponentToWorld` (`Actor.RootComponent` (`GameplayStatics.GetPlayerCharacter` 0))) "Undefined" "MultiplyWithRoot" null null))
  (`AIBlueprintHelperLibrary.SimpleMoveToActor` (`self.GetController` _returnvalue) _returnvalue)
  (`self.K2_DestroyActor`))

(event `Add_Tree`)

(event `Grant_Life`)

(fn `UserConstructionScript`)