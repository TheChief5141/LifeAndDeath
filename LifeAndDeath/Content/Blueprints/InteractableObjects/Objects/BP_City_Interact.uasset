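; Clickable city object that the player can hit once with a Fire, Tree or Life power.
; Until used, clicks are forwarded to its BP_AI_Object_Controller; RunInteraction then applies the chosen power, locks further clicks and removes the Niagara component.
; Fire spawns a temporary effect at TwinLevelActor, then destroys both twin and self.
; Tree spawns a tree actor on itself, while Life drives its Sphere with a delayed, reversing timeline.
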(event `self.ReceiveBeginPlay`
  ;[1 1 1] When this box is clicked, call event within AI_Object_Controller, which creates UI element above it
  (add `self.OnClicked` (delegate `OnClicked_Event`)))

(event `OnClicked_Event` :!signature `self.OnClicked`
  (params (TouchedActor :type "Actor Object Reference") (ButtonPressed :type "Key Structure" :default "None"))
  ;[1 1 1] When this box is clicked, call event within AI_Object_Controller, which creates UI element above it
  (if (not (`self.hasInteracted`))
    (bind _asbp_ai_object_controller (cast `/Game/Blueprints/InteractableObjects/Objects/BP_AI_Object_Controller` (`self.GetController`)))
    (`/Game/Blueprints/InteractableObjects/Objects/BP_AI_Object_Controller.OnClicked_Event` _asbp_ai_object_controller self "LeftMouseButton")))

(event `/Game/Blueprints/InteractableObjects/Interfaces/BI_Interactable.RunInteraction`
  (params (PowerUsed :type Byte))
  (bind _niagara (`self.Niagara`))
  ;[1 1 1] When BP Interactable calls this, activate power depending on inputted index
  (switch `int` (`KismetMathLibrary.Conv_ByteToInt` PowerUsed)
    (:`1`
      (`self.Create_Fire` self)
      (set `self.hasInteracted` true)
      (`ActorComponent.K2_DestroyComponent` _niagara))
    (:`2`
      (`self.Add_Tree` self)
      (set `self.hasInteracted` true)
      (`ActorComponent.K2_DestroyComponent` _niagara))
    (:`3`
      (`self.Grant_Life` self)
      (set `self.hasInteracted` true)
      (`ActorComponent.K2_DestroyComponent` _niagara))))

(event `Create_Fire`
  (params (Clicked_Object :type "Pawn Object Reference"))
  (bind _twin_level_actor (`self.Twin_Level_Actor`))
  (bind (_returnvalue_location _returnvalue_rotation _returnvalue_scale) (`KismetMathLibrary.BreakTransform` (`SceneComponent.K2_GetComponentToWorld` (`Actor.RootComponent` _twin_level_actor))))
  ;[1 1 1] Using Fire power
  (bind _returnvalue (`|SpawnActorFromClass` "/Game/Blueprints/Powers/Fire/PZD_Power_Fire.PZD_Power_Fire_C" (`KismetMathLibrary.MakeTransform` _returnvalue_location _returnvalue_rotation _returnvalue_scale) "Undefined" "MultiplyWithRoot" null null))
  (`KismetSystemLibrary.Delay` 1.0)
  (`self.K2_DestroyActor` _returnvalue)
  (`KismetSystemLibrary.Delay` 0.2)
  (`self.K2_DestroyActor` _twin_level_actor)
  (`KismetSystemLibrary.Delay` 0.2)
  (`self.K2_DestroyActor` self))

(event `Add_Tree`
  (params (Clicked_Object :type "Pawn Object Reference"))
  (bind (_returnvalue_location _returnvalue_rotation _returnvalue_scale) (`KismetMathLibrary.BreakTransform` (`SceneComponent.K2_GetComponentToWorld` (`Actor.RootComponent` Clicked_Object))))
  ;[1 1 1] Using Tree power
  (`|SpawnActorFromClass` "/Game/Blueprints/Powers/Tree/PZD_Power_Tree.PZD_Power_Tree_C" (`KismetMathLibrary.MakeTransform` _returnvalue_location (`KismetMathLibrary.MakeRotFromZ` (`KismetMathLibrary.MakeVector` 0.0)) _returnvalue_scale) "Undefined" "MultiplyWithRoot" null null))

(event `Grant_Life`
  (params (Clicked_Object :type "Pawn Object Reference"))
  ;[1 1 1] Using Life power
  (`KismetSystemLibrary.PrintString` "running grant life")
  (bind (_direction _newtrack_0) (`Timeline|SimpleMovement` :!label _label)
    (:`Update`
      (`SceneComponent.K2_SetRelativeLocation` (`self.Sphere`) _newtrack_0 false false)
      (`KismetSystemLibrary.Delay` 10.0)
      (if (`self.IsLooping`)
        (set `self.IsLooping` false)
        (goto _label :!via `Reverse`)
        (else
          (set `self.IsLooping` true)
          (goto _label))))))

(fn `UserConstructionScript`)